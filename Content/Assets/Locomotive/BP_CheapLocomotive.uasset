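; Cheap locomotive Blueprint, a skeleton with no gameplay logic of its own.
; Lifecycle, possession, significance, camera, VFX update, collision and rerail events only forward to their parent implementations, as does derail hologram spawning.
; Movement input, train naming, impact and derail effects, and stop validation are empty.
; Honk begin/end notifications and short/danger honks call the parent, while BeginHonk, EndHonk and the honk multicasts are empty.
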(event Custom|Server_Leave)

(event Custom|InpAxisEvt_MoveRight_K2Node_InputAxisEvent_0
  (params (AxisValue :type Float%20%28single-precision%29)))

(event Custom|InpAxisEvt_MoveForward_K2Node_InputAxisEvent_1
  (params (AxisValue :type Float%20%28single-precision%29)))

(event Custom|UpdateTrainName)

(event Custom|BeginHonk
  (params (AllowAlternativeHonk :type Boolean)))

(event Custom|EndHonk)

(event Custom|MulticastOnHonkShort)

(event Custom|MulticastOnHonkDanger)

(event EventBeginPlay
  (|CallParentFunction))

(event Collision|EventActorBeginOverlap
  (params (OtherActor :type Actor%20Object%20Reference)))

(event EventOnHonkBegin
  (|CallParentFunction))

(event EventOnHonkEnd
  (|CallParentFunction))

(event EventHonkShort
  (|CallParentFunction))

(event EventHonkDanger
  (|CallParentFunction))

(event EventOnRerail
  (|CallParentFunction))

(event EventOnCollided
  (params (withVehicle :type FG%20Railroad%20Vehicle%20Object%20Reference) (impactVelocity :type Float%20%28single-precision%29) (isPrimaryEvent :type Boolean) (isDerailed :type Boolean))
  (|CallParentFunction withVehicle impactVelocity isPrimaryEvent isDerailed))

(event EventTick
  (params (DeltaSeconds :type Float%20%28single-precision%29)))

(event EventUnpossessed
  (params (OldController :type Controller%20Object%20Reference))
  (|CallParentFunction OldController))

(event EventPossessed
  (params (NewController :type Controller%20Object%20Reference))
  (|CallParentFunction NewController))

(event EventOnNameChanged
  (|CallParentFunction))

(event EventGainedSignificance
  (|CallParentFunction))

(event EventLostSignificance
  (|CallParentFunction))

(event EventUpdateCamera
  (params (DeltaTime :type Float%20%28single-precision%29))
  (|CallParentFunction DeltaTime))

(event EventUpdateVFX
  (|CallParentFunction))

(fn ConstructionScript)

(fn SpawnCollisionVFX
  (params (ImpactForceScale :type Float%20%28single-precision%29)))

(fn EasterEgg
  (params (NewParam :type Float%20%28single-precision%29)))

(fn PlayLocomotiveImpactSFX
  (params (ImpactForce :type Float%20%28single-precision%29)))

(fn SpawnDeRailVFX
  (params (Location :type Vector) (Velocity :type Float%20%28single-precision%29) (forwardVector :type Vector) (Surface :type EPhysicalSurface%20Enum :default "SurfaceType_Default")))

(fn CheckValidationforStop)

(fn PlayLocomotiveImpact&DerailSFX
  (params (ImpactForce :type Float%20%28single-precision%29)))

(fn CheckActorVelocity)

(fn IsPossessed
  (bind _returnvalue (|CallParentFunction))
  (return _returnvalue))

(fn SpawnDerailHologram
  (params (transform :type Transform))
  (bind _returnvalue (|CallParentFunction transform))
  (return _returnvalue))